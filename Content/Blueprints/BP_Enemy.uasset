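; BP_Enemy is a melee enemy that chases the player once they enter its detection radius, using a self-repeating AI MoveTo.
; A looping one-second timer triggers an attack montage with delayed damage while the player is inside the attack radius.
; Incoming damage spawns a Niagara effect, and at zero health the enemy ragdolls and loses its health widget.
; Tick rotates that widget toward the player and updates its bar.
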(event `self.ReceiveBeginPlay`
  (set `self.CurrentHealth` (`self.MaxHealth`))
  (`KismetSystemLibrary.RetriggerableDelay` 1.0 :!label _label)
  (`self.Attack Player`)
  (goto _label))

(event `Chase Player`
  (if (not (`self.isDead`))
    (`|AIMoveTo` self (0.0 0.0 0.0) (`GameplayStatics.GetPlayerCharacter` 0) 120.0
      (:`OnSuccess`
        (`self.Chase Player`)))))

(event `self.DetectionRadius.OnComponentBeginOverlap`
  (params (OverlappedComponent :type "PrimitiveComponent Object Reference") (OtherActor :type "Actor Object Reference") (OtherComp :type "PrimitiveComponent Object Reference") (OtherBodyIndex :type Integer) (bFromSweep :type Boolean) (SweepResult :type "HitResult Structure (by ref)"))
  ;[1 1 1] Detection System
  (cast `/Game/ThirdPerson/Blueprints/BP_ThirdPersonCharacter` OtherActor)
  (`self.Chase Player`))

(event `self.ReceiveAnyDamage`
  (params (Damage :type "Float (single-precision)") (DamageType :type "DamageType Object Reference") (InstigatedBy :type "Controller Object Reference") (DamageCauser :type "Actor Object Reference"))
  ;[1 1 1] Health and DamageReceived
  (bind _output_get (set `self.CurrentHealth` (- (`self.CurrentHealth`) Damage)))
  (`NiagaraFunctionLibrary.SpawnSystemAtLocation` "/Game/NiagaraSystems/NS_Damage.NS_Damage" (`self.K2_GetActorLocation`) (struct) (1.0 1.0 1.0) true true "AutoRelease")
  (if (<= _output_get 0.0)
    (`PrimitiveComponent.SetSimulatePhysics` (`self.Mesh`) true)
    (`MovementComponent.StopMovementImmediately` (`self.CharacterMovement`))
    (set `self.isDead` true)
    (`ActorComponent.K2_DestroyComponent` (`self.HealthWidget`))))

(event `self.AttackRadius.OnComponentBeginOverlap`
  (params (OverlappedComponent :type "PrimitiveComponent Object Reference") (OtherActor :type "Actor Object Reference") (OtherComp :type "PrimitiveComponent Object Reference") (OtherBodyIndex :type Integer) (bFromSweep :type Boolean) (SweepResult :type "HitResult Structure (by ref)"))
  (cast `/Game/ThirdPerson/Blueprints/BP_ThirdPersonCharacter` OtherActor)
  (set `self.isInRadius` true))

(event `self.AttackRadius.OnComponentEndOverlap`
  (params (OverlappedComponent :type "PrimitiveComponent Object Reference") (OtherActor :type "Actor Object Reference") (OtherComp :type "PrimitiveComponent Object Reference") (OtherBodyIndex :type Integer))
  (cast `/Game/ThirdPerson/Blueprints/BP_ThirdPersonCharacter` OtherActor)
  (set `self.isInRadius` false))

(event `Attack Player`
  (if (and (`self.isInRadius`) (not (`self.isDead`)))
    (`self.PlayAnimMontage` "/Game/EnemyAnimations/Enemy_Attack_Montage.Enemy_Attack_Montage")
    (`KismetSystemLibrary.Delay` 0.22)
    (bind _asbp_third_person_character (cast `/Game/ThirdPerson/Blueprints/BP_ThirdPersonCharacter` (`GameplayStatics.GetPlayerCharacter` 0)))
    (`GameplayStatics.ApplyDamage` _asbp_third_person_character 1.0)))

(event `self.ReceiveTick`
  (params (DeltaSeconds :type "Float (single-precision)"))
  (bind _healthwidget (`self.HealthWidget`))
  (if (not (`self.isDead`))
    (`SceneComponent.K2_SetWorldRotation` _healthwidget (`KismetMathLibrary.FindLookAtRotation` (`SceneComponent.K2_GetComponentLocation` _healthwidget) (`self.K2_GetActorLocation` (`GameplayStatics.GetPlayerCharacter` 0))) false false)
    (bind _aswb_enemy_healthbar (cast `/Game/UserInterface/WB_EnemyHealthbar` (`WidgetComponent.GetWidget` (`self.HealthWidget`))))
    (set `ProgressBar.Percent` (/ (`self.CurrentHealth`) (`self.MaxHealth`)) (`/Game/UserInterface/WB_EnemyHealthbar.ProgressBar_0` _aswb_enemy_healthbar))))

(fn `UserConstructionScript`)